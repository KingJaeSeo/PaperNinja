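; A pressure-switch actor that sinks its mesh when something begins overlapping its box trigger.
; A timeline lerps the mesh's relative location downward, calling OnTurnedOn when it finishes forward and OnTurnedOff when it finishes backward.
; Momentary switches reverse the timeline when an overlap ends, and a TurnOff event can reverse it at any time.
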(event `self.ReceiveBeginPlay`)

(event `self.BoxTrigger.OnComponentBeginOverlap`
  (params (OverlappedComponent :type "PrimitiveComponent Object Reference") (OtherActor :type "Actor Object Reference") (OtherComp :type "PrimitiveComponent Object Reference") (OtherBodyIndex :type Integer) (bFromSweep :type Boolean) (SweepResult :type "HitResult Structure (by ref)"))
  (bind (_direction _alpha) (`Timeline|SwitchTimeLine` :!label _label)
    (:`Update`
      (`SceneComponent.K2_SetRelativeLocation` (`self.Mesh`) (`KismetMathLibrary.VLerp` (0.0 0.0 0.0) (0.0 0.0 -8.0) _alpha) false false))
    (:`Finished`
      (switch `ETimelineDirection` _direction
        (:`Forward`
          (`self.OnTurnedOn`))
        (:`Backward`
          (`self.OnTurnedOff`))))))

(event `self.BoxTrigger.OnComponentEndOverlap`
  (params (OverlappedComponent :type "PrimitiveComponent Object Reference") (OtherActor :type "Actor Object Reference") (OtherComp :type "PrimitiveComponent Object Reference") (OtherBodyIndex :type Integer))
  (if (`self.IsMomentary`)
    (goto _label :!via `Reverse`)))

(event `TurnOff`
  (goto _label :!via `Reverse`))

(fn `UserConstructionScript`)