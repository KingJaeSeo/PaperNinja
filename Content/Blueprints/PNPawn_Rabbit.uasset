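; PNPawn_Rabbit is a rabbit character that deals heavy damage to any actor its capsule hits.
; It starts at walk speed, and BeginSprint and EndSprint switch movement speed and the sprint flag.
; CanSeePlayerPawn line-traces forward by SightLength with debug drawing and checks for the "Player" tag.
; The sight check's debug print is disconnected, and nothing in this graph calls the sprint functions.
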(event `self.CapsuleComponent.OnComponentHit`
  (params (HitComponent :type "PrimitiveComponent Object Reference") (OtherActor :type "Actor Object Reference") (OtherComp :type "PrimitiveComponent Object Reference") (NormalImpulse :type "Vector Structure") (Hit :type "HitResult Structure (by ref)"))
  (`GameplayStatics.ApplyDamage` OtherActor 100.0))

(event `self.ReceiveBeginPlay`
  (set `CharacterMovementComponent.MaxWalkSpeed` (`self.WalkGroundSpeed`) (`self.CharacterMovement`)))

(event `self.ReceiveTick`
  (params (DeltaSeconds :type "Float (single-precision)")))

(fn `BeginSprint`
  (set `CharacterMovementComponent.MaxWalkSpeed` (`self.SprintGroundSpeed`) (`self.CharacterMovement`))
  (set `self.IsSprint` true))

(fn `CanSeePlayerPawn`
  (returns (ReturnValue :type Boolean) (SeenActor :type "Actor Object Reference"))
  (bind _returnvalue (`self.K2_GetActorLocation`))
  (bind _outhit (`KismetSystemLibrary.LineTraceSingle` :`Start` _returnvalue :`End` (+ _returnvalue (* (`self.GetActorForwardVector`) (`self.Sight Length`))) :`TraceChannel` "TraceTypeQuery3" :`DrawDebugType` "ForOneFrame"))
  (return (`self.ActorHasTag` (`.HitActor` (`GameplayStatics.BreakHitResult` _outhit)) "Player") null))

(fn `EndSprint`
  (set `CharacterMovementComponent.MaxWalkSpeed` (`self.WalkGroundSpeed`) (`self.CharacterMovement`))
  (set `self.IsSprint` false))

(fn `UserConstructionScript`)